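; Game mode Blueprint that tracks connected players and handles login validation for player controllers.
; PostLogin stores each PlayerControllerBP and assigns an incrementing index, while logout unpossesses its pawn and removes it; the minimum-player check triggers nothing yet.
; Validate checks credentials, rejects names already in the connected list, then re-adds the controller, sets its login and calls back with the result.
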(event Custom|Validate
  (params (Login :type String) (Password :type String) (PlayerController :type Player%20Controller%20BP%20Object%20Reference))
  (bind _returnvalue (Game|GetGameMode))
  (if (Class|IOFile|ValidateLogin Login Password)
    (bind _asgame_mode_bp (Utilities|Casting|CastToGameModeBP (Game|GetGameMode)))
    (bind _array_element (Utilities|Array|ForEachLoopwithBreak (Variables|GameModeBP_C|GetConnectedPlayers _asgame_mode_bp) :!label _label)
      (:LoopBody
        (if (Utilities|Enum|Equal(Enum) (Variables|/Game/Player/PlayerControllerBP.PlayerControllerBP_C|GetLogin _array_element) Login)
          (Variables|Default|SetIsLogged true)
          (goto _label Break)
          (else
            (Variables|Default|SetIsLogged false))))
      (:Completed
        (Development|PrintString (Utilities|GetDisplayName _returnvalue))
        (if (Variables|Default|GetIsLogged)
          (Default|UserLogged PlayerController)
          (else
            (bind _asgame_mode_bp_2 (Utilities|Casting|CastToGameModeBP _returnvalue)
              (:then
                (bind _returnvalue_2 (Utilities|Array|Add (Variables|GameModeBP_C|GetConnectedPlayers _asgame_mode_bp_2) PlayerController))
                (Variables|/Game/Player/PlayerControllerBP.PlayerControllerBP_C|SetLogin (Utilities|Array|Get(acopy) (Variables|GameModeBP_C|GetConnectedPlayers _asgame_mode_bp_2) _returnvalue_2) Login)
                (Development|PrintString (Utilities|String|ToString(Integer) (Utilities|Array|Length (Variables|GameModeBP_C|GetConnectedPlayers _asgame_mode_bp_2))))
                (Default|ValidationSuccesful PlayerController)
                (Default|AddPoints PlayerController))
              (:CastFailed
                (Development|PrintString "Hello")))))))
    (else
      (Default|ValidationFailure PlayerController))))

(event Custom|SetPlayerIndex
  (params (Player :type Player%20Controller%20BP%20Object%20Reference))
  (Variables|/Game/Player/PlayerControllerBP.PlayerControllerBP_C|SetIndex Player (Variables|Default|GetPlayersIndex))
  (Math|Integer|IncrementInt (Variables|Default|GetPlayersIndex)))

(event EventBeginPlay)

(event EventOnLogout
  (params (ExitingController :type Controller%20Object%20Reference))
  (bind _asplayer_controller_bp (Utilities|Casting|CastToPlayerControllerBP ExitingController))
  (Default|UnpossesPawn _asplayer_controller_bp)
  (Utilities|Array|RemoveItem (Variables|Default|GetConnectedPlayers) _asplayer_controller_bp))

(event EventPostLogin
  (params (NewPlayer :type Player%20Controller%20Object%20Reference))
  (bind _asplayer_controller_bp (Utilities|Casting|CastToPlayerControllerBP NewPlayer))
  (Utilities|Array|Add (Variables|Default|GetConnectedPlayers) _asplayer_controller_bp)
  (CallFunction|SetPlayerIndex _asplayer_controller_bp)
  (bind _returnvalue (Class|GameModeBase|GetNumPlayers))
  (Development|PrintString (Utilities|String|ToString(Integer) _returnvalue))
  (if (>= _returnvalue (Variables|Default|GetMinimumPlayers))
    _))

(fn ConstructionScript)