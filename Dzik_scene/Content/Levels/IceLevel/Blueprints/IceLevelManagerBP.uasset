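; Level manager for the Ice level that spawns and possesses each player's pawn when the level begins.
; On the server it spawns one IceLevelPlayer per starting player at tagged IceLevelStartingPoint actors, recording owner login, alive list and a back-reference to itself.
; After a short delay, each player gets the Slowka widget, possesses its pawn and switches view to the passed-in level camera.
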(event Custom|BeginLevel
  (params (Camera :type Actor%20Object%20Reference))
  (Networking|SwitchHasAuthority
    (:Authority
      (Variables|Default|SetCamera Camera)
      (CallFunction|SpawnPlayers)
      (Utilities|FlowControl|Delay 0.2)
      (CallFunction|PossesPawns))))

(event Custom|SpawnPlayers
  ;[1 1 1] Create Pawns
  (Networking|SwitchHasAuthority
    (:Authority
      (bind _outactors (Actor|GetAllActorswithTag "IceLevelStartingPoint"))
      (for _array_element (Variables|Default|GetStartingPlayers)
        (bind _returnvalue (Game|SpawnActorfromClass "/Game/Player/IceLevelPlayer.IceLevelPlayer_C" (Math|Conversions|ToTransform(Vector) (Transformation|GetActorLocation (Utilities|Array|Get(acopy) _outactors (Variables|Default|GetSpawningPointIndex)))) "Undefined" 0 0))
        (Variables|/Game/Player/IceLevelPlayer.IceLevelPlayer_C|SetPossesedBy _returnvalue (Variables|/Game/Player/PlayerControllerBP.PlayerControllerBP_C|GetLogin _array_element))
        (Utilities|Array|Add (Variables|Default|GetAlivePlayers) _returnvalue)
        (Variables|/Game/Player/PlayerControllerBP.PlayerControllerBP_C|SetToPossess _array_element _returnvalue)
        (Math|Integer|IncrementInt (Variables|Default|GetSpawningPointIndex)
          (:%20%20
            (CallFunction|SetIceManagerLevel _returnvalue self)))))))

(event Custom|SetIceManagerLevel
  (params (Player :type Ice%20Level%20Player%20Object%20Reference) (Manager :type Ice%20Level%20Manager%20BP%20Object%20Reference))
  ;[1 1 1] Create Pawns
  (Variables|/Game/Player/IceLevelPlayer.IceLevelPlayer_C|SetIceLevelManager Player Manager))

(event Custom|PossesPawns
  ;[1 1 1] Posses Pawns
  (for _array_element (Variables|Default|GetStartingPlayers)
    (Default|ActivateSlowkaWidget _array_element)
    (Default|PossessPawn _array_element)
    (Default|ChangeView _array_element (Variables|Default|GetCamera))))

(fn ConstructionScript)