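; Player Blueprint that tracks whether the player holds the kielbasa and carries click-to-move logic marked as deprecated.
; On left click, the non-authority branch passes the controller and cursor hit to a custom event, and both call SimpleMoveToLocation toward that point.
; GetKielbasa and LoseKielbasa set the GotKielbasa flag and swap the mesh material between CubeMaterial and CustomDepth to show possession.
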(event Custom|CustomEvent
  (params (NewParam :type Controller%20Object%20Reference) (NewParam2 :type Hit%20Result%20Structure))
  ;[1 1 1] Old version of moving/ Deprecated
  (AI|Navigation|SimpleMovetoLocation NewParam (.Location (Collision|BreakHitResult NewParam2))))

(event Collision|EventActorBeginOverlap
  (params (OtherActor :type Actor%20Object%20Reference)))

(event Input|MouseEvents|LeftMouseButton
  (params (Key :type Key%20Structure :default "None"))
  ;[1 1 1] Old version of moving/ Deprecated
  (:Pressed
    (bind _asplayer_controller_bp (Utilities|Casting|CastToPlayerControllerBP (Pawn|GetController)))
    (Networking|SwitchHasAuthority
      (:Remote
        (CallFunction|CustomEvent _asplayer_controller_bp (.HitResult (Game|Player|GetHitResultUnderCursorbyChannel _asplayer_controller_bp "TraceTypeQuery1" true)))
        (AI|Navigation|SimpleMovetoLocation _asplayer_controller_bp (.Location (Collision|BreakHitResult (.HitResult (Game|Player|GetHitResultUnderCursorbyChannel _asplayer_controller_bp "TraceTypeQuery1" true)))))))))

(fn ConstructionScript)

(fn GetKielbasa
  (Variables|Default|SetGotKielbasa true)
  (Rendering|Material|SetMaterial (Variables|Character|GetMesh) 0 "/Engine/EngineMaterials/CubeMaterial.CubeMaterial"))

(fn LoseKielbasa
  (Variables|Default|SetGotKielbasa false)
  (Rendering|Material|SetMaterial (Variables|Character|GetMesh) 0 "/Engine/BufferVisualization/CustomDepth.CustomDepth"))