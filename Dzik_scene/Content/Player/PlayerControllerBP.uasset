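; Player controller Blueprint that manages level UI, login validation, server connection and pawn possession.
; BeginPlay caps FPS at 60 and pre-creates boar, Slowka, points, countdown, instruction and settings widgets, which paired events show or hide.
; ServerValidate passes credentials to GameModeBP, and result events update the main menu or clear all widgets.
; Other events handle delayed possession and blended view changes; a login-menu test is unwired.
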(event Custom|UserLogged
  (bind _foundwidgets (Widget|GetAllWidgetsOfClass "/Game/Main_Menu/Main_menu_widget.Main_menu_widget_C" false))
  (Default|UserLogged _foundwidgets))

(event Custom|ValidationFailure
  (bind _foundwidgets (Widget|GetAllWidgetsOfClass "/Game/Main_Menu/Main_menu_widget.Main_menu_widget_C" false))
  (Default|ValidationRetry _foundwidgets))

(event Custom|UnpossesPawn
  (Pawn|UnPossess))

(event Custom|DeactivateBoarWidget
  ;[1 1 1] WidgetsControl
  (Widget|RemovefromParent (Variables|Default|GetBoarLevelWidget)))

(event Custom|ActivatePointsWidget
  ;[1 1 1] WidgetsControl
  (UserInterface|Viewport|AddtoViewport (Variables|Default|GetPointsWidget) 0))

(event Custom|AddToPointsList
  (params (PointsEntry :type Points%20Info%20Structure))
  ;[1 1 1] WidgetsControl
  (Default|AddtoList (Variables|Default|GetPointsWidget) PointsEntry))

(event Custom|UpdatePointList
  (params (NewList :type Array%20of%20Points%20Info%20Structures))
  ;[1 1 1] WidgetsControl
  (Default|RemoveList (Variables|Default|GetPointsWidget))
  (CallFunction|AddListtoPoints NewList))

(event Custom|ActivateSlowkaWidget
  (bind _slowkalevelwidget (Variables|Default|GetSlowkaLevelWidget))
  ;[1 1 1] WidgetsControl
  (UserInterface|Viewport|AddtoViewport _slowkalevelwidget 0)
  (Default|SettFocus _slowkalevelwidget)
  (Variables|Default|SetSlowkaActivated true))

(event Custom|ActivateCountdownWidget
  ;[1 1 1] WidgetsControl
  (UserInterface|Viewport|AddtoViewport (Variables|Default|GetCountdownWidget) 0))

(event Custom|AddListToPoints
  (params (List :type Array%20of%20Points%20Info%20Structures))
  ;[1 1 1] WidgetsControl
  (Default|AddList (Variables|Default|GetPointsWidget) List))

(event Custom|DeactivateCountdownWidget
  ;[1 1 1] WidgetsControl
  (Widget|RemovefromParent (Variables|Default|GetCountdownWidget)))

(event Custom|StartCountdown
  (params (Time :type Integer))
  ;[1 1 1] WidgetsControl
  (CallFunction|ActivateCountdownWidget)
  (Default|Countdown (Variables|Default|GetCountdownWidget) Time))

(event Custom|ValidationSuccesful
  (Viewport|RemoveAllWidgets))

(event Custom|ActivateInstruction
  ;[1 1 1] WidgetsControl
  (UserInterface|Viewport|AddtoViewport (Variables|Default|GetLevelInstruction) 0))

(event Custom|ActivateSetting
  ;[1 1 1] WidgetsControl
  (UserInterface|Viewport|AddtoViewport (Variables|Default|GetSettingsWidget) 0))

(event Custom|DeactivateSlowkaWdiget
  (bind _slowkalevelwidget (Variables|Default|GetSlowkaLevelWidget))
  ;[1 1 1] WidgetsControl
  (Default|Reset _slowkalevelwidget)
  (Widget|RemovefromParent _slowkalevelwidget)
  (Variables|Default|SetSlowkaActivated false))

(event Custom|DeactivateInstruction
  ;[1 1 1] WidgetsControl
  (Widget|RemovefromParent (Variables|Default|GetLevelInstruction)))

(event Custom|ChangeInstruction
  (params (Instruction :type String))
  ;[1 1 1] WidgetsControl
  (Default|ChangeText (Variables|Default|GetLevelInstruction) Instruction))

(event Custom|DeactiveSetting
  ;[1 1 1] WidgetsControl
  (Widget|RemovefromParent (Variables|Default|GetSettingsWidget)))

(event Custom|ActivateSettingsButton
  ;[1 1 1] WidgetsControl
  (UserInterface|Viewport|AddtoViewport (Variables|Default|GetSettingsButtonWidget) 0))

(event Custom|DeactivateSettingsButton
  ;[1 1 1] WidgetsControl
  (Widget|RemovefromParent (Variables|Default|GetSettingsButtonWidget)))

(event Custom|Disable
  (AI|Navigation|StopMovement))

(event Custom|ShowSettings
  (Utilities|FlowControl|FlipFlop
    (:A
      (CallFunction|ActivateSetting))
    (:B
      (CallFunction|DeactiveSetting))))

(event Custom|ConnectToIP
  (params (IP :type Text))
  (Game|OpenLevel(byName) (Utilities|String|StringToName (Utilities|String|ToString(Text) IP))))

(event Custom|ServerValidate
  (params (Login :type String) (Password :type String))
  (bind _asgame_mode_bp (Utilities|Casting|CastToGameModeBP (Game|GetGameMode)))
  (Default|Validate _asgame_mode_bp Login Password self))

(event Custom|DeactivatePointsWidget
  ;[1 1 1] WidgetsControl
  (Widget|RemovefromParent (Variables|Default|GetPointsWidget)))

(event Custom|AddPoints
  (params (Player1 :type String) (Player2 :type String) (Player3 :type String))
  (bind _returnvalue (UserInterface|CreateWidget "/Game/Player/Widgets/PointsWdiget.PointsWdiget_C"))
  (Utilities|Array|Add (Variables|Default|GetWidgetsList) _returnvalue)
  (UserInterface|Viewport|AddtoViewport _returnvalue 0))

(event Custom|ChangeView
  (params (NewView :type Actor%20Object%20Reference))
  (Utilities|FlowControl|Delay 1.0)
  (Game|Player|SetViewTargetwithBlend NewView 1.0 "VTBlend_Linear" 0.0 false))

(event Custom|ActivateBoarWidget
  ;[1 1 1] WidgetsControl
  (UserInterface|Viewport|AddtoViewport (Variables|Default|GetBoarLevelWidget) 0))

(event Custom|PossessPawn
  (Utilities|FlowControl|Delay 0.2)
  (Pawn|Possess self (Variables|Default|GetToPossess)))

(event EventBeginPlay
  (Development|ExecuteConsoleCommand "t.maxfps 60" 0)
  (Variables|Default|SetbShowMouseCursor true)
  (bind _returnvalue (UserInterface|CreateWidget "/Game/Player/Widgets/BoarLevelWidget.BoarLevelWidget_C"))
  (Variables|Default|SetBoarLevelWidget _returnvalue)
  (bind _returnvalue_2 (UserInterface|CreateWidget "/Game/Player/Widgets/PointsWdiget.PointsWdiget_C"))
  (Variables|Default|SetPointsWidget _returnvalue_2)
  (bind _returnvalue_3 (UserInterface|CreateWidget "/Game/Player/Widgets/CountDown.CountDown_C"))
  (Variables|Default|SetCountdownWidget _returnvalue_3)
  (bind _returnvalue_4 (UserInterface|CreateWidget "/Game/Player/Widgets/SlowkaLevelWidget.SlowkaLevelWidget_C"))
  (Variables|Default|SetSlowkaLevelWidget _returnvalue_4)
  (bind _returnvalue_5 (UserInterface|CreateWidget "/Game/Player/Widgets/LevelInstruction.LevelInstruction_C"))
  (Variables|Default|SetLevelInstruction _returnvalue_5)
  (bind _returnvalue_6 (UserInterface|CreateWidget "/Game/Player/Widgets/SettingsButtonWidget.SettingsButtonWidget_C"))
  (Variables|Default|SetSettingsButtonWidget _returnvalue_6)
  (CallFunction|ActivateSettingsButton)
  (bind _returnvalue_7 (UserInterface|CreateWidget "/Game/Player/Widgets/SettingsWidget.SettingsWidget_C"))
  (Variables|Default|SetSettingsWidget _returnvalue_7))

(fn ConstructionScript)